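; Enemy character that chases the player and plays a punch montage on reaching them.
; PawnSensing sightings start an AI MoveTo toward the player and reset a DoOnce, which gates the montage when the move succeeds.
; The construction script snaps a Sphere to the left toe socket and attaches it to the mesh.
; Damage and capsule overlaps with the player's Sphere only print debug messages.
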(event `self.ReceiveBeginPlay`)

(event `self.ReceiveTick`
  (params (DeltaSeconds :type "Float (single-precision)")))

(event `self.PawnSensing.OnSeePawn`
  (params (Pawn :type "Pawn Object Reference"))
  (set `self.isSeePlayer?` true)
  (`self.FollowCharater`)
  (goto _label :!via `Reset`))

(event `FollowCharater`
  (if (`self.isSeePlayer?`)
    (`|AIMoveTo` self (0.0 0.0 0.0) (`GameplayStatics.GetPlayerCharacter` 0) 200.0
      (:`OnSuccess`
        (`/Engine/EditorBlueprintResources/StandardMacros.DoOnce` false :!label _label
          (:`Completed`
            (`self.PlayAnimMontage` "/Game/Enemy/PunchAnimMontage.PunchAnimMontage")))))))

(event `self.CapsuleComponent.OnComponentBeginOverlap`
  (params (OverlappedComponent :type "PrimitiveComponent Object Reference") (OtherActor :type "Actor Object Reference") (OtherComp :type "PrimitiveComponent Object Reference") (OtherBodyIndex :type Integer) (bFromSweep :type Boolean) (SweepResult :type "HitResult Structure (by ref)"))
  (bind _asbp_third_person_character (cast `/Game/ThirdPerson/Blueprints/BP_ThirdPersonCharacter` (`GameplayStatics.GetPlayerCharacter` 0))
    (:`then`
      (if (== OtherComp (`/Game/ThirdPerson/Blueprints/BP_ThirdPersonCharacter.Sphere` _asbp_third_person_character))
        (`KismetSystemLibrary.PrintString` "sdsad")))
    (:`CastFailed`
      (`KismetSystemLibrary.PrintString` "cast fail"))))

(event `self.Sphere.OnComponentBeginOverlap`
  (params (OverlappedComponent :type "PrimitiveComponent Object Reference") (OtherActor :type "Actor Object Reference") (OtherComp :type "PrimitiveComponent Object Reference") (OtherBodyIndex :type Integer) (bFromSweep :type Boolean) (SweepResult :type "HitResult Structure (by ref)")))

(event `self.ReceiveAnyDamage`
  (params (Damage :type "Float (single-precision)") (DamageType :type "DamageType Object Reference") (InstigatedBy :type "Controller Object Reference") (DamageCauser :type "Actor Object Reference"))
  (`KismetSystemLibrary.PrintString` "Hasar" true true (struct :`R` 1.0 :`G` 0.204922 :`A` 1.0)))

(fn `UserConstructionScript`
  (`SceneComponent.K2_SetWorldLocation` (`self.Sphere`) (`SceneComponent.GetSocketLocation` (`self.Mesh`) "LeftToeBaseSocket") false false)
  (`SceneComponent.K2_AttachToComponent` (`self.Sphere`) (`self.Mesh`) "None" "KeepWorld" "KeepWorld" "KeepWorld" true))