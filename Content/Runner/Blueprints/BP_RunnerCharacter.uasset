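; BP_RunnerCharacter is a player character that runs forward automatically and jumps on input.
; On BeginPlay it adds the IMC_RunnerDefault Enhanced Input mapping context to the owning player controller's subsystem.
; Tick applies constant movement input along the control rotation's yaw, so running follows the controller's facing without any movement input from the player.
; The Jump_IA action triggers the standard character Jump.
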(event `self.ReceiveBeginPlay`
  ;[1 1 1] Comment
  (bind _asplayer_controller (cast `PlayerController` (`self.GetController`)))
  (bind _returnvalue (pcsubsystem `EnhancedInputLocalPlayerSubsystem` _asplayer_controller))
  (`/Engine/EditorBlueprintResources/StandardMacros.IsValid` _returnvalue
    (:`Is Valid`
      (`EnhancedInputSubsystemInterface.AddMappingContext` _returnvalue "/Game/Runner/Blueprints/IMC_RunnerDefault.IMC_RunnerDefault" 0 (struct)))))

(event `self.ReceiveTick`
  (params (DeltaSeconds :type "Float (single-precision)"))
  ;[1 1 1] Comment
  (`self.AddMovementInput` (`KismetMathLibrary.GetForwardVector` (`KismetMathLibrary.MakeRotator` 0.0 0.0 (.yaw (`self.GetControlRotation`))))))

(event `EnhancedInput|/Game/Runner/Blueprints/Jump_IA`
  (params (ActionValue :type Boolean) (ElapsedSeconds :type "Float (double-precision)") (TriggeredSeconds :type "Float (double-precision)") (InputAction :type "InputAction Object Reference" :default "/Game/Runner/Blueprints/Jump_IA.Jump_IA"))
  (:`Triggered`
    (`self.Jump`)))

(fn `UserConstructionScript`)