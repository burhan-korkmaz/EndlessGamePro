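; BP_Obstackles_Wall is a runner-game wall obstacle that kills the player and can be destroyed by damage.
; On actor overlap, it casts to BP_RunnerCharacter and calls its DeathEvent.
; AnyDamage stores Damage minus Healt back into Healt (operands reversed from usual subtraction), prints it, then recomputes that difference and destroys the wall at zero or below.
; An unconnected Death, delay and pause chain never runs.
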(event `self.ReceiveActorBeginOverlap`
  (params (OtherActor :type "Actor Object Reference"))
  (bind _asbp_runner_character (cast `/Game/Runner/Blueprints/BP_RunnerCharacter` OtherActor))
  (`/Game/Runner/Blueprints/BP_RunnerCharacter.DeathEvent` _asbp_runner_character))

(event `self.ReceiveAnyDamage`
  (params (Damage :type "Float (single-precision)") (DamageType :type "DamageType Object Reference") (InstigatedBy :type "Controller Object Reference") (DamageCauser :type "Actor Object Reference"))
  (bind _returnvalue (- Damage (`self.Healt`)))
  (set `self.Healt` _returnvalue)
  (`KismetSystemLibrary.PrintString` (`KismetStringLibrary.Conv_DoubleToString` (`self.Healt`)))
  (if (<= _returnvalue 0.0)
    (`self.K2_DestroyActor`)))

(fn `UserConstructionScript`
  (`parent.UserConstructionScript`))