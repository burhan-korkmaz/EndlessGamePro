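; BP_Floor_2 is a runner floor piece with moving side walls and a damage box.
; From BeginPlay, a self-restarting timeline nudges both walls in opposite Y directions relative to their current positions.
; When the player overlaps the box, it prints a debug message and subtracts health stored on BP_RunnerGamemode.
; Functions for building lane spawn points and randomly spawning child-actor obstacles exist but are not called here.
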(event `self.ReceiveBeginPlay`
  (`self.CustomEvent`)
  (bind _asbp_runner_gamemode (cast `/Game/Runner/Blueprints/BP_RunnerGamemode` (`GameplayStatics.GetGameMode`)))
  (set `self.As BP Runner Gamemode` _asbp_runner_gamemode))

(event `self.ReceiveTick`
  (params (DeltaSeconds :type "Float (single-precision)")))

(event `CustomEvent`
  (bind _rightwall (`self.RightWall`))
  (bind _leftwall (`self.LeftWall`))
  (bind (_returnvalue_x _returnvalue_y _returnvalue_z) (`KismetMathLibrary.BreakVector` (`SceneComponent.K2_GetComponentLocation` (`self.RightWall`))))
  (bind (_returnvalue_x_2 _returnvalue_y_2 _returnvalue_z_2) (`KismetMathLibrary.BreakVector` (`SceneComponent.K2_GetComponentLocation` (`self.LeftWall`))))
  (bind (_direction _newtrack_0) (`Timeline|Timeline` :!via `PlayFromStart`)
    (:`Update`
      (`SceneComponent.K2_SetWorldLocation` _leftwall (`KismetMathLibrary.VLerp` (`SceneComponent.K2_GetComponentLocation` _leftwall) (`KismetMathLibrary.MakeVector` _returnvalue_x_2 (+ _returnvalue_y_2 0.3) _returnvalue_z_2) _newtrack_0) false false)
      (`SceneComponent.K2_SetWorldLocation` _rightwall (`KismetMathLibrary.VLerp` (`SceneComponent.K2_GetComponentLocation` _rightwall) (`KismetMathLibrary.MakeVector` _returnvalue_x (+ _returnvalue_y -0.3) _returnvalue_z) _newtrack_0) false false))
    (:`Finished`
      (`self.CustomEvent`))))

(event `self.Box.OnComponentBeginOverlap`
  (params (OverlappedComponent :type "PrimitiveComponent Object Reference") (OtherActor :type "Actor Object Reference") (OtherComp :type "PrimitiveComponent Object Reference") (OtherBodyIndex :type Integer) (bFromSweep :type Boolean) (SweepResult :type "HitResult Structure (by ref)"))
  (bind _as_bp_runner_gamemode (`self.As BP Runner Gamemode`))
  (bind _asbp_third_person_character (cast `/Game/ThirdPerson/Blueprints/BP_ThirdPersonCharacter` (`GameplayStatics.GetPlayerCharacter` 0)))
  (if (== OtherActor _asbp_third_person_character)
    (`KismetSystemLibrary.PrintString` "Hello")
    (set `/Game/Runner/Blueprints/BP_RunnerGamemode.CharacterHealth` (- (`/Game/Runner/Blueprints/BP_RunnerGamemode.CharacterHealth` _as_bp_runner_gamemode) 10) _as_bp_runner_gamemode)))

(fn `GetAttachPoint`)

(fn `SetupSpawnPositions`
  (for _array_element (`self.LanePosition`)
    (for _index (range 2)
      (bind _returnvalue (`AddComponent|NODE_AddArrowComponent-0` :`RelativeTransform` (`KismetMathLibrary.MakeTransform` (`KismetMathLibrary.MakeVector` (* _index 650.0) _array_element))))
      (`KismetArrayLibrary.Array_Add` (`self.SpawnPoints`) (`SceneComponent.K2_GetComponentToWorld` _returnvalue)))))

(fn `SpawnObstackles`
  (bind _output_get (set `self.RandomSpawnPoints` (`self.SpawnPoints`)))
  (`KismetArrayLibrary.Array_Shuffle` _output_get)
  (for _index (range (+ (`KismetMathLibrary.RandomIntegerInRange` 0 2) 1))
    (switch `int` (`KismetMathLibrary.RandomIntegerInRange` 0 1)
      (:`0`
        (bind _returnvalue (`KismetMathLibrary.MakeRelativeTransform` (`|GetArrayItem` (`self.RandomSpawnPoints`) _index) (`self.GetTransform`)))
        (`AddComponent|NODE_AddChildActorComponent-0` :`RelativeTransform` _returnvalue))
      (:`1`
        (`AddComponent|NODE_AddChildActorComponent-1` :`RelativeTransform` _returnvalue)))))

(fn `UserConstructionScript`)